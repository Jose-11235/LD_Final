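; BP_PlayChar is the player character, handling movement, look, jump, shooting, dashing and health, with game over triggered through BP_PlayCon.
; Enhanced Input drives actions: shooting spawns projectiles from the Cube on a half-second cooldown.
; Dash launches along current horizontal velocity on release, scaled by hold time.
; SpawnDash and SpawnKey each spawn a one-time pickup when shoot or bite kill counts reach their thresholds.
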(event `EnhancedInput|/Game/BP/Input/IA_Jump`
  (params (ActionValue :type Boolean) (ElapsedSeconds :type "Float (double-precision)") (TriggeredSeconds :type "Float (double-precision)") (InputAction :type "InputAction Object Reference" :default "/Game/BP/Input/IA_Jump.IA_Jump"))
  ; Basic Movement
  (:`Started`
    (`self.Jump`)))

(event `self.ReceiveAnyDamage`
  (params (Damage :type "Float (single-precision)") (DamageType :type "DamageType Object Reference") (InstigatedBy :type "Controller Object Reference") (DamageCauser :type "Actor Object Reference"))
  (bind _health (`self.Health`))
  ; Damage
  (set `self.Health` (- _health Damage))
  (if (<= _health 0.0)
    (bind _asbp_play_con (cast `/Game/BP/Framework/BP_PlayCon` (`GameplayStatics.GetPlayerController` 0)))
    (`/Game/BP/Framework/BP_PlayCon.GameOver` _asbp_play_con)))

(event `EnhancedInput|/Game/BP/Input/IA_Locomotion`
  (params (ActionValue :type "Float (double-precision)") (ElapsedSeconds :type "Float (double-precision)") (TriggeredSeconds :type "Float (double-precision)") (InputAction :type "InputAction Object Reference" :default "/Game/BP/Input/IA_Locomotion.IA_Locomotion"))
  ; Basic Movement
  (:`Triggered`
    (`self.AddMovementInput` (`self.GetActorForwardVector`) ActionValue)))

(event `EnhancedInput|/Game/BP/Input/IA_Strafing`
  (params (ActionValue :type "Float (double-precision)") (ElapsedSeconds :type "Float (double-precision)") (TriggeredSeconds :type "Float (double-precision)") (InputAction :type "InputAction Object Reference" :default "/Game/BP/Input/IA_Strafing.IA_Strafing"))
  ; Basic Movement
  (:`Triggered`
    (`self.AddMovementInput` (`self.GetActorRightVector`) ActionValue)))

(event `EnhancedInput|/Game/BP/Input/IA_LookH`
  (params (ActionValue :type "Float (double-precision)") (ElapsedSeconds :type "Float (double-precision)") (TriggeredSeconds :type "Float (double-precision)") (InputAction :type "InputAction Object Reference" :default "/Game/BP/Input/IA_LookH.IA_LookH"))
  ; Basic Movement
  (:`Triggered`
    (`self.AddControllerYawInput` ActionValue)))

(event `EnhancedInput|/Game/BP/Input/IA_LookV`
  (params (ActionValue :type "Float (double-precision)") (ElapsedSeconds :type "Float (double-precision)") (TriggeredSeconds :type "Float (double-precision)") (InputAction :type "InputAction Object Reference" :default "/Game/BP/Input/IA_LookV.IA_LookV"))
  ; Basic Movement
  (:`Triggered`
    (`self.AddControllerPitchInput` ActionValue)))

(event `EnhancedInput|/Game/BP/Input/IA_Shooting`
  (params (ActionValue :type Boolean) (ElapsedSeconds :type "Float (double-precision)") (TriggeredSeconds :type "Float (double-precision)") (InputAction :type "InputAction Object Reference" :default "/Game/BP/Input/IA_Shooting.IA_Shooting"))
  ; Shoot
  (:`Started`
    (if (`self.CanShoot`)
      (`/Engine/EditorBlueprintResources/StandardMacros.DoOnce` false :!label _label
        (:`Completed`
          (`|SpawnActorFromClass` "/Game/BP/Gameplay/BP_Projectile.BP_Projectile_C" (`SceneComponent.K2_GetComponentToWorld` (`self.Cube`)) "Undefined" "MultiplyWithRoot" null null)
          (`KismetSystemLibrary.Delay` 0.5)
          (goto _label :!via `Reset`))))))

(event `EnhancedInput|/Game/BP/Input/IA_Dash`
  (params (ActionValue :type Boolean) (ElapsedSeconds :type "Float (double-precision)") (TriggeredSeconds :type "Float (double-precision)") (InputAction :type "InputAction Object Reference" :default "/Game/BP/Input/IA_Dash.IA_Dash"))
  (bind (_returnvalue_x _returnvalue_y) (`KismetMathLibrary.BreakVector` (* (`self.GetVelocity`) (`self.DashForce`))))
  ; Dash
  (:`Completed`
    (if (`self.CanDash`)
      (set `self.DashForce` (`KismetMathLibrary.Lerp` 10.0 50.0 (`KismetMathLibrary.FClamp` (`KismetMathLibrary.NormalizeToRange` ElapsedSeconds 0.0 1.0))))
      (set `self.IsDashing` true)
      (`self.LaunchCharacter` (`KismetMathLibrary.MakeVector` _returnvalue_x _returnvalue_y) true)
      (`KismetSystemLibrary.Delay` 0.5)
      (set `self.IsDashing` false))))

(event `SpawnDash`
  ; Dash Unlock
  (if (== (`self.ShootKill`) 3)
    (`/Engine/EditorBlueprintResources/StandardMacros.DoOnce` false
      (:`Completed`
        (`|SpawnActorFromClass` "/Game/BP/Gameplay/Checks/BP_DashUnlock.BP_DashUnlock_C" (`self.GetTransform`) "AlwaysSpawn" "MultiplyWithRoot" null null)))))

(event `SpawnKey`
  ; Spawn Key
  (if (== (`self.BiteKill`) 5)
    (`/Engine/EditorBlueprintResources/StandardMacros.DoOnce` false
      (:`Completed`
        (`|SpawnActorFromClass` "/Game/BP/Gameplay/Checks/BP_BellKey.BP_BellKey_C" (`self.GetTransform`) "AlwaysSpawn" "MultiplyWithRoot" null null)))))

(fn `UserConstructionScript`)