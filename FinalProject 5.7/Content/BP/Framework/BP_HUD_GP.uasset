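; BP_HUD_GP is the gameplay HUD Blueprint that owns the player's screen widgets.
; On BeginPlay it creates the pause, HUD, health bar, game over and level clear widgets for player 0, stores references and adds them to the player screen.
; All start collapsed except the health bar, which is visible without intercepting input itself.
; An UpdateObjectiveText event forwards objective text and duration to the HUD widget.
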(event `self.ReceiveBeginPlay`
  (bind _returnvalue (`GameplayStatics.GetPlayerController` 0))
  (`|ExecutionSequence`
    (:`then_0`
      (bind _returnvalue_2 (`|CreateWidget` "/Game/BP/UI/WBP_PauseScreen.WBP_PauseScreen_C" _returnvalue))
      (bind _output_get (set `self.PauseRef` _returnvalue_2))
      (`UserWidget.AddToPlayerScreen` _output_get 0)
      (`Widget.SetVisibility` _output_get "Collapsed"))
    (:`then_1`
      (bind _returnvalue_3 (`|CreateWidget` "/Game/BP/UI/WBP_HUD.WBP_HUD_C" _returnvalue))
      (bind _output_get_2 (set `self.HUDRef` _returnvalue_3))
      (`UserWidget.AddToPlayerScreen` _output_get_2 0)
      (`Widget.SetVisibility` _output_get_2 "Collapsed"))
    (:`then_2`
      (bind _returnvalue_4 (`|CreateWidget` "/Game/BP/UI/WBP_HealthBar.WBP_HealthBar_C" _returnvalue))
      (bind _output_get_3 (set `self.HealthRef` _returnvalue_4))
      (`UserWidget.AddToPlayerScreen` _output_get_3 0)
      (`Widget.SetVisibility` _output_get_3 "SelfHitTestInvisible"))
    (:`then_3`
      (bind _returnvalue_5 (`|CreateWidget` "/Game/BP/UI/WBP_GameOver.WBP_GameOver_C" _returnvalue))
      (bind _output_get_4 (set `self.GameOverRef` _returnvalue_5))
      (`UserWidget.AddToPlayerScreen` _output_get_4 0)
      (`Widget.SetVisibility` _output_get_4 "Collapsed"))
    (:`then_4`
      (bind _returnvalue_6 (`|CreateWidget` "/Game/BP/UI/WBP_LevelClear.WBP_LevelClear_C" _returnvalue))
      (bind _output_get_5 (set `self.LevelClearRef` _returnvalue_6))
      (`UserWidget.AddToPlayerScreen` _output_get_5 0)
      (`Widget.SetVisibility` _output_get_5 "Collapsed"))))

(event `/Game/BP/Utilities/BPI_HUDUpdates.UpdateObjectiveText`
  (params (ObjectiveText :type Text) (Duration :type "Float (double-precision)"))
  (`/Game/BP/UI/WBP_HUD.UpdateObjective` (`self.HUDRef`) ObjectiveText Duration))

(fn `UserConstructionScript`)