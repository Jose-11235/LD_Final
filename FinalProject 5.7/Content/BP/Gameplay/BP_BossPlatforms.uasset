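; Boss-fight platform that projectiles move between Start and End, counting toward the boss's defeat.
; An UpTrigger hit relocates that trigger to Start and plays a transform-lerp timeline.
; A DownTrigger hit restores UpTrigger to UpPivot, increments this platform's Counter and reverses the timeline.
; Once Counter reaches three, timeline updates repeatedly call BossDefeated, snap WinRef's pivot to its End and update the HUD objective.
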(event `self.UpTrigger.OnComponentBeginOverlap`
  (params (OverlappedComponent :type "PrimitiveComponent Object Reference") (OtherActor :type "Actor Object Reference") (OtherComp :type "PrimitiveComponent Object Reference") (OtherBodyIndex :type Integer) (bFromSweep :type Boolean) (SweepResult :type "HitResult Structure (by ref)"))
  (bind _winref (`self.WinRef`))
  (cast `/Game/BP/Gameplay/BP_Projectile` OtherActor)
  (`SceneComponent.K2_SetWorldTransform` (`self.UpTrigger`) (`SceneComponent.K2_GetComponentToWorld` (`self.Start`)) false false)
  (bind (_direction _kinematic_timeline) (`Timeline|Timeline` :!label _label)
    (:`Update`
      (`SceneComponent.K2_SetWorldTransform` (`self.Pivot`) (`KismetMathLibrary.TLerp` (`SceneComponent.K2_GetComponentToWorld` (`self.Start`)) (`SceneComponent.K2_GetComponentToWorld` (`self.End`)) _kinematic_timeline) false false)
      (if (>= (`self.Counter`) 3.0)
        (`/Game/BP/Gameplay/Enemies/BP_Boss.BossDefeated` (`self.BossRef`))
        (`SceneComponent.K2_SetWorldTransform` (`/Game/BP/Gameplay/Checks/BP_WinUnlock.Pivot` _winref) (`SceneComponent.K2_GetComponentToWorld` (`/Game/BP/Gameplay/Checks/BP_WinUnlock.End` _winref)) false false)
        (message `/Game/BP/Utilities/BPI_HUDUpdates.UpdateObjectiveText` (`PlayerController.GetHUD` (`GameplayStatics.GetPlayerController` 0)) "Get a Tooth from the Beast as proof for the Guild" 2.0)))))

(event `self.DownTrigger.OnComponentBeginOverlap`
  (params (OverlappedComponent :type "PrimitiveComponent Object Reference") (OtherActor :type "Actor Object Reference") (OtherComp :type "PrimitiveComponent Object Reference") (OtherBodyIndex :type Integer) (bFromSweep :type Boolean) (SweepResult :type "HitResult Structure (by ref)"))
  (cast `/Game/BP/Gameplay/BP_Projectile` OtherActor)
  (`SceneComponent.K2_SetWorldTransform` (`self.UpTrigger`) (`SceneComponent.K2_GetComponentToWorld` (`self.UpPivot`)) false false)
  (set `self.Counter` (+ (`self.Counter`) 1.0))
  (goto _label :!via `Reverse`))

(fn `UserConstructionScript`)