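; BP_EnemyBite is a chest-monster enemy that chases the player on sight and bites on contact.
; PawnSensing triggers the attack animation and AI MoveTo toward BP_PlayChar.
; A capsule hit from a dashing player destroys it immediately; otherwise it deals bite sound and damage after a short delay.
; When destroyed, it increments the player's BiteKill count and calls SpawnKey on the player.
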(event `self.PawnSensing.OnSeePawn`
  (params (Pawn :type "Pawn Object Reference"))
  (bind _asbp_play_char (cast `/Game/BP/Framework/BP_PlayChar` Pawn))
  (`SkeletalMeshComponent.PlayAnimation` (`self.ChestMonster_SK`) "/Game/MonsterForSurvivalGame/Animation/PBR/ChestMonster/ChestMonster_Attack01_ANIM.ChestMonster_Attack01_ANIM" false)
  (`|AIMoveTo` self (0.0 0.0 0.0) _asbp_play_char 5.0 true))

(event `self.CapsuleComponent.OnComponentHit`
  (params (HitComponent :type "PrimitiveComponent Object Reference") (OtherActor :type "Actor Object Reference") (OtherComp :type "PrimitiveComponent Object Reference") (NormalImpulse :type "Vector Structure") (Hit :type "HitResult Structure (by ref)"))
  (bind _asbp_play_char (cast `/Game/BP/Framework/BP_PlayChar` OtherActor))
  (if (`/Game/BP/Framework/BP_PlayChar.IsDashing` _asbp_play_char)
    (`SkeletalMeshComponent.PlayAnimation` (`self.ChestMonster_SK`) "/Game/MonsterForSurvivalGame/Animation/PBR/ChestMonster/ChestMonster_Die_ANIM.ChestMonster_Die_ANIM" false)
    (`self.K2_DestroyActor`)
    (else
      (`KismetSystemLibrary.Delay` 0.4)
      (`GameplayStatics.PlaySoundAtLocation` "/Game/Sound/SFX_EnemyBite.SFX_EnemyBite" (`self.K2_GetActorLocation`) (struct) 1.0 1.0 0.0 null null null null)
      (`GameplayStatics.ApplyDamage` _asbp_play_char 1.0))))

(event `self.ReceiveDestroyed`
  (bind _asbp_play_char (cast `/Game/BP/Framework/BP_PlayChar` (`GameplayStatics.GetPlayerCharacter` 0)))
  (`/Engine/EditorBlueprintResources/StandardMacros.IncrementInt` (`/Game/BP/Framework/BP_PlayChar.BiteKill` _asbp_play_char)
    (:`  `
      (`/Game/BP/Framework/BP_PlayChar.SpawnKey` _asbp_play_char))))

(fn `UserConstructionScript`)