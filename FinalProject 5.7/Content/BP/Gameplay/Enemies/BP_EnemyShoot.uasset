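; Mushroom enemy that turns to face the player on sight and fires projectiles.
; Pawn sensing loops the attack animation, rotates the actor and capsule toward the player, and spawns BP_EnemyProjectile at its spawn point with a sound.
; A CanAttack flag and short delay throttle the fire rate.
; On destruction it increments the player's ShootKill count and calls the player's SpawnDash.
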(event `self.PawnSensing.OnSeePawn`
  (params (Pawn :type "Pawn Object Reference"))
  (bind _asbp_play_char (cast `/Game/BP/Framework/BP_PlayChar` Pawn))
  (`SkeletalMeshComponent.PlayAnimation` (`self.Mushroom_SK`) "/Game/MonsterForSurvivalGame/Animation/PBR/Mushroom/SmileVersion/Mushroom_Attack01Smile_ANIM.Mushroom_Attack01Smile_ANIM" true)
  (bind _returnvalue (`KismetMathLibrary.FindLookAtRotation` (`self.K2_GetActorLocation`) (`self.K2_GetActorLocation` _asbp_play_char)))
  (`self.K2_SetActorRotation` _returnvalue)
  (`SceneComponent.K2_SetWorldRotation` (`self.CapsuleComponent`) _returnvalue false false)
  (if (`self.CanAttack`)
    (`GameplayStatics.PlaySoundAtLocation` "/Game/Sound/SFX_EnemyShoot.SFX_EnemyShoot" (`self.K2_GetActorLocation`) (struct) 1.0 1.0 0.0 null null null null)
    (`|SpawnActorFromClass` "/Game/BP/Gameplay/Enemies/BP_EnemyProjectile.BP_EnemyProjectile_C" (`SceneComponent.K2_GetComponentToWorld` (`self.ProjectileSpawnPoint`)) "Undefined" "MultiplyWithRoot" null null)
    (set `self.CanAttack` false)
    (`KismetSystemLibrary.Delay` 0.45)
    (set `self.CanAttack` true)))

(event `self.ReceiveDestroyed`
  (bind _asbp_play_char (cast `/Game/BP/Framework/BP_PlayChar` (`GameplayStatics.GetPlayerCharacter` 0)))
  (`/Engine/EditorBlueprintResources/StandardMacros.IncrementInt` (`/Game/BP/Framework/BP_PlayChar.ShootKill` _asbp_play_char)
    (:`  `
      (`/Game/BP/Framework/BP_PlayChar.SpawnDash` _asbp_play_char))))

(fn `UserConstructionScript`)