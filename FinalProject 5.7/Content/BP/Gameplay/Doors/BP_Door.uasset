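; BP_Door is a door actor that opens when a BP_PlayChar with BellUnlocked set enters its trigger.
; A timeline moves the Pivot component by interpolating its world transform between the Start and End components.
; Without the unlock, the HUD shows a timed "Locked" objective message instead.
; The file contains no closing logic.
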(event `self.Trigger.OnComponentBeginOverlap`
  (params (OverlappedComponent :type "PrimitiveComponent Object Reference") (OtherActor :type "Actor Object Reference") (OtherComp :type "PrimitiveComponent Object Reference") (OtherBodyIndex :type Integer) (bFromSweep :type Boolean) (SweepResult :type "HitResult Structure (by ref)"))
  (bind _asbp_play_char (cast `/Game/BP/Framework/BP_PlayChar` OtherActor))
  (if (`/Game/BP/Framework/BP_PlayChar.BellUnlocked` _asbp_play_char)
    (bind (_direction _kinematictimeline) (`Timeline|KinematicTimeline`)
      (:`Update`
        (`SceneComponent.K2_SetWorldTransform` (`self.Pivot`) (`KismetMathLibrary.TLerp` (`SceneComponent.K2_GetComponentToWorld` (`self.Start`)) (`SceneComponent.K2_GetComponentToWorld` (`self.End`)) _kinematictimeline) false false)))
    (else
      (message `/Game/BP/Utilities/BPI_HUDUpdates.UpdateObjectiveText` (`PlayerController.GetHUD` (`GameplayStatics.GetPlayerController` 0)) "Locked" 3.0))))

(fn `UserConstructionScript`)