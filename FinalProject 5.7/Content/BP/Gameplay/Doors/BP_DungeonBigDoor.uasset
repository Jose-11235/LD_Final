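; BP_DungeonBigDoor is a large dungeon gate that projectiles open by hitting two triggers.
; The first hit bumps a counter and destroys that trigger, and a hit with the counter at two plays the timeline.
; The timeline lerps Pivot between Start and End transforms, with a one-time gate sound on its first update.
; A player entering CloseTrigger reverses the timeline, or plays it forward if CanWin is set.
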(event `self.Trigger.OnComponentBeginOverlap`
  (params (OverlappedComponent :type "PrimitiveComponent Object Reference") (OtherActor :type "Actor Object Reference") (OtherComp :type "PrimitiveComponent Object Reference") (OtherBodyIndex :type Integer) (bFromSweep :type Boolean) (SweepResult :type "HitResult Structure (by ref)"))
  (cast `/Game/BP/Gameplay/BP_Projectile` OtherActor)
  (if (== (`self.Counter`) 2)
    (bind (_direction _kinematictimeline) (`Timeline|Timeline_0` :!label _label)
      (:`Update`
        (`SceneComponent.K2_SetWorldTransform` (`self.Pivot`) (`KismetMathLibrary.TLerp` (`SceneComponent.K2_GetComponentToWorld` (`self.Start`)) (`SceneComponent.K2_GetComponentToWorld` (`self.End`)) _kinematictimeline) false false)
        (`/Engine/EditorBlueprintResources/StandardMacros.DoOnce` false
          (:`Completed`
            (`GameplayStatics.PlaySoundAtLocation` "/Game/Sound/SFX_DungeonGate.SFX_DungeonGate" (`self.K2_GetActorLocation`) (struct) 1.0 1.0 0.0 null null null null)))))
    (else
      (set `self.Counter` (+ (`self.Counter`) 2))
      (`ActorComponent.K2_DestroyComponent` (`self.Trigger`)))))

(event `self.Trigger1.OnComponentBeginOverlap`
  (params (OverlappedComponent :type "PrimitiveComponent Object Reference") (OtherActor :type "Actor Object Reference") (OtherComp :type "PrimitiveComponent Object Reference") (OtherBodyIndex :type Integer) (bFromSweep :type Boolean) (SweepResult :type "HitResult Structure (by ref)"))
  (cast `/Game/BP/Gameplay/BP_Projectile` OtherActor)
  (if (== (`self.Counter`) 2)
    (goto _label)
    (else
      (set `self.Counter` (+ (`self.Counter`) 2))
      (`ActorComponent.K2_DestroyComponent` (`self.Trigger1`)))))

(event `self.CloseTrigger.OnComponentBeginOverlap`
  (params (OverlappedComponent :type "PrimitiveComponent Object Reference") (OtherActor :type "Actor Object Reference") (OtherComp :type "PrimitiveComponent Object Reference") (OtherBodyIndex :type Integer) (bFromSweep :type Boolean) (SweepResult :type "HitResult Structure (by ref)"))
  (bind _asbp_play_char (cast `/Game/BP/Framework/BP_PlayChar` OtherActor))
  (if (`/Game/BP/Framework/BP_PlayChar.CanWin` _asbp_play_char)
    (goto _label)
    (else
      (goto _label :!via `Reverse`))))

(fn `UserConstructionScript`)