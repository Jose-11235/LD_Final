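; Boss enemy that shoots projectiles at the player character and damages it on contact.
; When PawnSensing sees the player, it rotates the projectile spawn point toward them and spawns a boss projectile, gated by a CanAttack flag that resets after a short delay.
; A hit on the Sphere component by the player applies damage after a brief delay, with no cooldown gate.
; An unconnected node for disabling sensing never runs.
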(event `self.PawnSensing.OnSeePawn`
  (params (Pawn :type "Pawn Object Reference"))
  (bind _asbp_play_char (cast `/Game/BP/Framework/BP_PlayChar` Pawn))
  (`SceneComponent.K2_SetWorldRotation` (`self.ProjectileSpawnPoint`) (`KismetMathLibrary.FindLookAtRotation` (`self.K2_GetActorLocation`) (`self.K2_GetActorLocation` _asbp_play_char)) false false)
  (if (`self.CanAttack`)
    (`|SpawnActorFromClass` "/Game/BP/Gameplay/Enemies/BP_BossProjectile.BP_BossProjectile_C" (`SceneComponent.K2_GetComponentToWorld` (`self.ProjectileSpawnPoint`)) "Undefined" "MultiplyWithRoot" null null)
    (set `self.CanAttack` false)
    (`KismetSystemLibrary.Delay` 0.5)
    (set `self.CanAttack` true)))

(event `self.Sphere.OnComponentHit`
  (params (HitComponent :type "PrimitiveComponent Object Reference") (OtherActor :type "Actor Object Reference") (OtherComp :type "PrimitiveComponent Object Reference") (NormalImpulse :type "Vector Structure") (Hit :type "HitResult Structure (by ref)"))
  (bind _asbp_play_char (cast `/Game/BP/Framework/BP_PlayChar` OtherActor))
  (`KismetSystemLibrary.Delay` 0.5)
  (`GameplayStatics.ApplyDamage` _asbp_play_char 1.0))

(fn `UserConstructionScript`)