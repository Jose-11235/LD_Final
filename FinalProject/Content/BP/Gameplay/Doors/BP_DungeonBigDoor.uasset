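; A large dungeon door that opens once projectiles have hit its two triggers and closes when the player character enters a close trigger.
; The first trigger hit raises a shared counter and destroys that trigger, so a hit on the remaining one finds the counter at its threshold and plays the timeline.
; The timeline lerps the door pivot between start and end transforms, and the close trigger reverses it.
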(event `self.Trigger.OnComponentBeginOverlap`
  (params (OverlappedComponent :type "PrimitiveComponent Object Reference") (OtherActor :type "Actor Object Reference") (OtherComp :type "PrimitiveComponent Object Reference") (OtherBodyIndex :type Integer) (bFromSweep :type Boolean) (SweepResult :type "HitResult Structure (by ref)"))
  (cast `/Game/BP/Gameplay/BP_Projectile` OtherActor)
  (if (== (`self.Counter`) 2)
    (bind (_direction _kinematictimeline) (`Timeline|Timeline_0` :!label _label)
      (:`Update`
        (`SceneComponent.K2_SetWorldTransform` (`self.Pivot`) (`KismetMathLibrary.TLerp` (`SceneComponent.K2_GetComponentToWorld` (`self.Start`)) (`SceneComponent.K2_GetComponentToWorld` (`self.End`)) _kinematictimeline) false false)))
    (else
      (set `self.Counter` (+ (`self.Counter`) 2))
      (`ActorComponent.K2_DestroyComponent` (`self.Trigger`)))))

(event `self.Trigger1.OnComponentBeginOverlap`
  (params (OverlappedComponent :type "PrimitiveComponent Object Reference") (OtherActor :type "Actor Object Reference") (OtherComp :type "PrimitiveComponent Object Reference") (OtherBodyIndex :type Integer) (bFromSweep :type Boolean) (SweepResult :type "HitResult Structure (by ref)"))
  (cast `/Game/BP/Gameplay/BP_Projectile` OtherActor)
  (if (== (`self.Counter`) 2)
    (goto _label)
    (else
      (set `self.Counter` (+ (`self.Counter`) 2))
      (`ActorComponent.K2_DestroyComponent` (`self.Trigger1`)))))

(event `self.CloseTrigger.OnComponentBeginOverlap`
  (params (OverlappedComponent :type "PrimitiveComponent Object Reference") (OtherActor :type "Actor Object Reference") (OtherComp :type "PrimitiveComponent Object Reference") (OtherBodyIndex :type Integer) (bFromSweep :type Boolean) (SweepResult :type "HitResult Structure (by ref)"))
  (cast `/Game/BP/Framework/BP_PlayChar` OtherActor)
  (goto _label :!via `Reverse`))

(fn `UserConstructionScript`)