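; BP_DungeonGate is a dungeon gate that opens when a BP_Projectile overlaps its Trigger component.
; The overlap plays a Timeline that interpolates the Pivot's world transform from the Start component to the End component, without sweep.
; Each Timeline update also sets the player HUD's objective message to "Enter the Dungeon", so the message is re-sent throughout the movement.
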(event `self.Trigger.OnComponentBeginOverlap`
  (params (OverlappedComponent :type "PrimitiveComponent Object Reference") (OtherActor :type "Actor Object Reference") (OtherComp :type "PrimitiveComponent Object Reference") (OtherBodyIndex :type Integer) (bFromSweep :type Boolean) (SweepResult :type "HitResult Structure (by ref)"))
  (cast `/Game/BP/Gameplay/BP_Projectile` OtherActor)
  (bind (_direction _kinematictimeline) (`Timeline|Timeline`)
    (:`Update`
      (`SceneComponent.K2_SetWorldTransform` (`self.Pivot`) (`KismetMathLibrary.TLerp` (`SceneComponent.K2_GetComponentToWorld` (`self.Start`)) (`SceneComponent.K2_GetComponentToWorld` (`self.End`)) _kinematictimeline) false false)
      (message `/Game/BP/Utilities/BPI_HUDUpdates.UpdateObjectiveText` (`PlayerController.GetHUD` (`GameplayStatics.GetPlayerController` 0)) "Enter the Dungeon" 3.0))))

(fn `UserConstructionScript`)