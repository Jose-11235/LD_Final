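; BP_Sign is a trigger actor that shows a sign widget when the player character walks into it.
; The first overlap creates WBP_Sign, adds it to the player screen, and switches input to UI-only with the mouse cursor shown.
; The widget's close button is bound to an event that destroys the sign actor after a short delay, making it a one-time popup.
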(event `self.Trigger.OnComponentBeginOverlap`
  (params (OverlappedComponent :type "PrimitiveComponent Object Reference") (OtherActor :type "Actor Object Reference") (OtherComp :type "PrimitiveComponent Object Reference") (OtherBodyIndex :type Integer) (bFromSweep :type Boolean) (SweepResult :type "HitResult Structure (by ref)"))
  (bind _returnvalue (`GameplayStatics.GetPlayerController` 0))
  (if (== OtherActor (`GameplayStatics.GetPlayerCharacter` 0))
    (`/Engine/EditorBlueprintResources/StandardMacros.DoOnce` false
      (:`Completed`
        (bind _returnvalue_2 (`|CreateWidget` "/Game/BP/UI/WBP_Sign.WBP_Sign_C" _returnvalue))
        (bind _output_get (set `self.SignRef` _returnvalue_2))
        (`UserWidget.AddToPlayerScreen` _output_get 0)
        (`WidgetBlueprintLibrary.SetInputMode_UIOnlyEx` _returnvalue _output_get "DoNotLock" true)
        (set `PlayerController.bShowMouseCursor` true _returnvalue)
        (add `/Game/BP/UI/WBP_GameButton.BtnClicked` (`/Game/BP/UI/WBP_Sign.BtnClose` (`self.SignRef`)) (delegate `DestroyWidget`))))))

(event `DestroyWidget`
  (`KismetSystemLibrary.Delay` 1.0)
  (`self.K2_DestroyActor`))

(fn `UserConstructionScript`)